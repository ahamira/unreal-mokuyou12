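; BP_mydoor is a swinging door that BP_MyTestCharacter opens by entering its trigger box.
; It opens freely without a key name or switch flag; otherwise it requires the named key as Got and marks it Used.
; A timeline drives the mesh's yaw, then SetEventFinished calls its parent, saves event status to the game instance, fixes the open rotation and disables the box's collision.
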(event `self.Box.OnComponentBeginOverlap`
  (params (OverlappedComponent :type "PrimitiveComponent Object Reference") (OtherActor :type "Actor Object Reference") (OtherComp :type "PrimitiveComponent Object Reference") (OtherBodyIndex :type Integer) (bFromSweep :type Boolean) (SweepResult :type "HitResult Structure (by ref)"))
  (bind _asbp_my_test_character (cast `/Game/新規フォルダ/BP_MyTestCharacter` OtherActor))
  (if (and (== (`self.Key Name`) "None") (not (`self.swich mydoor`)))
    (`self.Open Door`)
    (else
      (switch `/Game/新規フォルダ/EN_MyKeyStatus` (`/Game/新規フォルダ/BP_MyTestCharacter.GetKeyStatus` _asbp_my_test_character (`self.Key Name`))
        (:`NewEnumerator1`
          (`/Game/新規フォルダ/BP_MyTestCharacter.UpdateMyKeyStatus` _asbp_my_test_character (`self.Key Name`) "NewEnumerator2")
          (`self.Open Door`))))))

(event `Open Door`
  (set `self.swich mydoor` false)
  (bind (_direction _openz) (`Timeline|Open1`)
    (:`Update`
      (`SceneComponent.K2_SetRelativeRotation` (`self.STM_mydoor`) (`KismetMathLibrary.MakeRotator` 0.0 0.0 _openz) false false))
    (:`Finished`
      (`self.SetEventFinished`))))

(event `self.ReceiveBeginPlay`
  (`parent.ReceiveBeginPlay`))

(fn `SetEventFinished`
  (`parent.SetEventFinished`)
  (`/Game/新規フォルダ/BP_My1GameInstance.SaveEventStatus` (`self.As BP My 1Game Instance`) (`self.EventName`) "NewEnumerator2")
  (set `self.swich mydoor` false)
  (`SceneComponent.K2_SetRelativeRotation` (`self.STM_mydoor`) (struct :`Yaw` 90.0) false false)
  (`PrimitiveComponent.SetCollisionEnabled` (`self.Box`) "NoCollision"))

(fn `UserConstructionScript`)
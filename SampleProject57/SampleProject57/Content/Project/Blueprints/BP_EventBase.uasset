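; Base Blueprint for game events that records a finished or unfinished status in BP_MyGameInstance.
; The construction script derives EventName from the object's display name, which serves as the key for that status.
; BeginPlay reads the stored status, calling SetEventFinished if it is Finished and otherwise saving it as Unfinished.
; SetEventFinished marks the event Finished and writes that back to the game instance.
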(event `self.ReceiveBeginPlay`
  (bind _asbp_my_game_instance (cast `/Game/Project/Blueprints/BP_MyGameInstance` (`GameplayStatics.GetGameInstance`)))
  (bind _output_get (set `self.MyGameInstance` _asbp_my_game_instance))
  (bind _output_get_2 (set `self.EventStatus` (`/Game/Project/Blueprints/BP_MyGameInstance.GetEventStatus` _output_get (`self.EventName`))))
  (switch `/Game/Project/Blueprints/EN_EventStatus` _output_get_2
    (:`NewEnumerator2`
      (bind _output_get_3 (set `self.EventStatus` "NewEnumerator0"))
      (`/Game/Project/Blueprints/BP_MyGameInstance.SaveEventStatus` (`self.MyGameInstance`) (`self.EventName`) _output_get_3))
    (:`NewEnumerator1`
      (`self.SetEventFinished`))))

(fn `SetEventFinished`
  (bind _output_get (set `self.EventStatus` "NewEnumerator1"))
  (`/Game/Project/Blueprints/BP_MyGameInstance.SaveEventStatus` (`self.MyGameInstance`) (`self.EventName`) _output_get))

(fn `UserConstructionScript`
  (set `self.EventName` (`KismetStringLibrary.Conv_StringToName` (`KismetSystemLibrary.GetDisplayName` self))))